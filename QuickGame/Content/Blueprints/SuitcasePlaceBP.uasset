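; SuitcasePlaceBP is an actor marking a placement spot, apparently for a suitcase, that can end the game.
; Any overlap with its Box reveals the Place component while IsPlaced is false, and ending an overlap hides it.
; If IsPlaced is true when an overlap ends, it also calls CompleteGame on the cached MyQuickGameMode.
; IsPlaced is only read here, never set.
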(event `self.ReceiveBeginPlay`
  (bind _asmy_quick_game_mode (cast `/Game/Blueprints/MyQuickGameMode` (`GameplayStatics.GetGameMode`)))
  (set `self.As My Quick Game Mode` _asmy_quick_game_mode))

(event `self.Box.OnComponentBeginOverlap`
  (params (OverlappedComponent :type "PrimitiveComponent Object Reference") (OtherActor :type "Actor Object Reference") (OtherComp :type "PrimitiveComponent Object Reference") (OtherBodyIndex :type Integer) (bFromSweep :type Boolean) (SweepResult :type "HitResult Structure (by ref)"))
  (if (not (`self.isPlaced`))
    (`SceneComponent.SetHiddenInGame` (`self.Place`) false false)))

(event `self.Box.OnComponentEndOverlap`
  (params (OverlappedComponent :type "PrimitiveComponent Object Reference") (OtherActor :type "Actor Object Reference") (OtherComp :type "PrimitiveComponent Object Reference") (OtherBodyIndex :type Integer))
  (bind _place (`self.Place`))
  (if (`self.isPlaced`)
    (`SceneComponent.SetHiddenInGame` _place true false)
    (`/Game/Blueprints/MyQuickGameMode.CompleteGame` (`self.As My Quick Game Mode`))
    (else
      (`SceneComponent.SetHiddenInGame` _place true false))))

(fn `UserConstructionScript`)