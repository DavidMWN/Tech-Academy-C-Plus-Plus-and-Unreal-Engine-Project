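; Game mode that handles the fail and win outcomes of a small level-based game.
; FallOff restarts play by opening MainMap, while CompleteGame shows the completion widget and sets IsComplete.
; It enables input from the first player controller on BeginPlay, so the game mode itself receives the Enter key, which quits the game once complete.
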(event `self.ReceiveBeginPlay`
  (`self.EnableInput` (`GameplayStatics.GetPlayerController` 0)))

(event `FallOff`
  (`GameplayStatics.OpenLevel` "MainMap"))

(event `CompleteGame`
  (bind _returnvalue (`|CreateWidget` "/Game/Blueprints/CompleteGameWidget.CompleteGameWidget_C"))
  (`UserWidget.AddToPlayerScreen` _returnvalue 0)
  (set `self.IsComplete` true))

(event `Key|Enter`
  (params (Key :type "Key Structure"))
  (:`Pressed`
    (if (`self.IsComplete`)
      (`KismetSystemLibrary.QuitGame` null "Quit"))))

(fn `UserConstructionScript`)